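; BP_Key is a rotatable lock-code piece that operates as a child of another actor.
; ToggleActivation disables the parent's player input, then plays a right or left timeline that adds yaw to LockCode1.
; Delays inside each timeline update gate the rotation and re-enable input afterwards.
; ToggleHighlight swaps the piece between normal and highlighted steel materials.
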(event `/Game/Blueprints/BPI_Activable.ToggleActivation`
  (params (bActivate :type Boolean))
  (bind _timelinelenght (`self.TimelineLenght`))
  (`self.DisableInput` (`self.GetParentActor`) (`GameplayStatics.GetPlayerController` 0))
  (if bActivate
    (bind (_direction _rotation) (`Timeline|Move Right` :`NewTime` _timelinelenght :!via `PlayFromStart`)
      (:`Update`
        (`KismetSystemLibrary.Delay` 0.2)
        (`SceneComponent.K2_AddLocalRotation` (`self.LockCode1`) (`KismetMathLibrary.MakeRotator` 0.0 0.0 _rotation) false false)
        (`KismetSystemLibrary.Delay` _timelinelenght)))
    (else
      (bind (_direction_2 _move_left) (`Timeline|Move Left` :`NewTime` _timelinelenght :!via `PlayFromStart`)
        (:`Update`
          (`KismetSystemLibrary.Delay` 0.2)
          (`SceneComponent.K2_AddLocalRotation` (`self.LockCode1`) (`KismetMathLibrary.MakeRotator` 0.0 0.0 _move_left) false false)
          (`KismetSystemLibrary.Delay` _timelinelenght)))))
  (`self.EnableInput` (`self.GetParentActor`) (`GameplayStatics.GetPlayerController` 0)))

(event `/Game/Blueprints/BPI_Highlightable.ToggleHighlight`
  (params (bActive :type Boolean))
  (bind _lockcode1 (`self.LockCode1`))
  (if bActive
    (`PrimitiveComponent.SetMaterial` _lockcode1 0 "/Game/StarterContent/Materials/M_Metal_Burnished_SteelHighlited.M_Metal_Burnished_SteelHighlited")
    (else
      (`PrimitiveComponent.SetMaterial` _lockcode1 0 "/Game/StarterContent/Materials/M_Metal_Burnished_Steel.M_Metal_Burnished_Steel"))))

(fn `UserConstructionScript`)