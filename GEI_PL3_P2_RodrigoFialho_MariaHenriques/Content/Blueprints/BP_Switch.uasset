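; BP_Switch is an interactable switch actor that responds to the E key while the player pawn stands inside its Box trigger.
; Box overlap begin and end events enable and disable input on the actor for the first player controller.
; Pressing E calls Turn with a fixed true value, so it only prints "On"; the "Off" branch is never reached from this graph.
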(event `self.Box.OnComponentBeginOverlap`
  (params (OverlappedComponent :type "PrimitiveComponent Object Reference") (OtherActor :type "Actor Object Reference") (OtherComp :type "PrimitiveComponent Object Reference") (OtherBodyIndex :type Integer) (bFromSweep :type Boolean) (SweepResult :type "HitResult Structure (by ref)"))
  (if (== OtherActor (`GameplayStatics.GetPlayerPawn` 0))
    (`self.EnableInput` (`GameplayStatics.GetPlayerController` 0))))

(event `self.Box.OnComponentEndOverlap`
  (params (OverlappedComponent :type "PrimitiveComponent Object Reference") (OtherActor :type "Actor Object Reference") (OtherComp :type "PrimitiveComponent Object Reference") (OtherBodyIndex :type Integer))
  (if (== OtherActor (`GameplayStatics.GetPlayerPawn` 0))
    (`self.DisableInput` (`GameplayStatics.GetPlayerController` 0))))

(event `Key|E`
  (params (Key :type "Key Structure"))
  (:`Pressed`
    (`self.Turn` true)))

(fn `Turn`
  (params (bOn :type Boolean))
  (if bOn
    (`KismetSystemLibrary.PrintString` "On")
    (else
      (`KismetSystemLibrary.PrintString` "Off")))
  (return))

(fn `UserConstructionScript`)