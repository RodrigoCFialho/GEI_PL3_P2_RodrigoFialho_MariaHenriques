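; BP_Lock is an interactive three-row combination lock that opens a linked stash.
; E toggles lock mode, blending to a static camera and disabling pawn input while the lock takes control.
; W/S select a highlighted row; A/D cycle its four-value icon through BPI_Activable child actors and recheck the code.
; A match plays the LockOpening timeline, marks it unlocked, restores player control and activates the stash.
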(event `self.ReceiveBeginPlay`
  (for (_array_element _array_index) (`self.Code`)
    (`KismetSystemLibrary.PrintString` (`KismetStringLibrary.Concat_StrStr` "Row:" (`KismetStringLibrary.Conv_IntToString` _array_index) "Code:" (`KismetStringLibrary.Conv_IntToString` _array_element)))))

(event `Key|E`
  (params (Key :type "Key Structure"))
  (bind _lockrotationpoint (`self.LockRotationPoint`))
  (bind _stash (`self.Stash`))
  (bind (_relativelocation_x _relativelocation_y) (`KismetMathLibrary.BreakVector` (`SceneComponent.RelativeLocation` _lockrotationpoint)))
  (:`Pressed`
    (if (`self.bWasUnlocked`)
      _
      (elif (`self.bIsActive`)
        (`self.Turn` false)
        (else
          (`self.Turn` true)
          ;[1 1 1] Opening Lock
          (bind _newparam2 (`self.CheckCode` :!label _label)
            (:`NewParam3`
              (bind (_direction _height _rotation) (`Timeline|LockOpening` :!via `PlayFromStart`)
                (:`Update`
                  (`SceneComponent.K2_SetRelativeLocationAndRotation` _lockrotationpoint (`KismetMathLibrary.MakeVector` _relativelocation_x _relativelocation_y _height) (`KismetMathLibrary.MakeRotator` 0.0 0.0 _rotation) false false))
                (:`Finished`
                  (`self.ToggleOpenText`
                    (:`Out`
                      (set `self.bWasUnlocked` true)
                      (`self.Interact` false
                        (:`Out`
                          ;[1 1 1] Open stash
                          (`/Engine/EditorBlueprintResources/StandardMacros.IsValid` _stash
                            (:`Is Valid`
                              (bind _asbpi_activable (cast `/Game/Blueprints/BPI_Activable` _stash)
                                (:`then`
                                  (`/Game/Blueprints/BPI_Activable.ToggleActivation` _asbpi_activable _newparam2))
                                (:`CastFailed`
                                  (`KismetSystemLibrary.PrintString` "FAIL!"))))))))))))))))))

(event `Key|S`
  (params (Key :type "Key Structure"))
  (:`Pressed`
    (if (`self.bIsActive`)
      (`self.MoveDown`))))

(event `Key|W`
  (params (Key :type "Key Structure"))
  (:`Pressed`
    (if (`self.bIsActive`)
      (`self.MoveUp`))))

(event `Key|D`
  (params (Key :type "Key Structure"))
  (:`Pressed`
    (if (`self.bIsActive`)
      (`self.MoveRight`
        (:`Out`
          (goto _label))))))

(event `Key|A`
  (params (Key :type "Key Structure"))
  (:`Pressed`
    (if (`self.bIsActive`)
      (`self.MoveLeft`
        (:`Out`
          (goto _label))))))

(event `/Game/Blueprints/BPI_Activable.ToggleActivation`
  (params (bActivate :type Boolean))
  (bind _returnvalue (`GameplayStatics.GetPlayerController` 0))
  (bind _transitiontime (`self.TransitionTime`))
  (if bActivate
    (`self.ToggleCharacterMovement` false
      (:`Out`
        (`self.ChangeViewToStaticCamera`)
        (`KismetSystemLibrary.Delay` _transitiontime)
        (`self.EnableInput` _returnvalue)
        (`self.ActivateLock` bActivate)))
    (else
      (`self.DisableInput` _returnvalue)
      (`self.ChangeViewToControllerCamera`)
      (`KismetSystemLibrary.Delay` _transitiontime)
      (`self.EnableInput` _returnvalue)
      (`self.ToggleCharacterMovement` true
        (:`Out`
          (`self.DeactivateLock` false))))))

(fn `Turn`
  (params (bOn :type Boolean))
  (`parent.Turn` bOn)
  (`self.Interact` bOn))

(fn `UserConstructionScript`
  (bind _lockcoderow (`self.LockCodeRow`))
  (`KismetArrayLibrary.Array_Clear` _lockcoderow)
  (`KismetArrayLibrary.Array_Add` _lockcoderow (`self.ChildActor`))
  (`KismetArrayLibrary.Array_Add` _lockcoderow (`self.ChildActor1`))
  (`KismetArrayLibrary.Array_Add` _lockcoderow (`self.ChildActor2`)))