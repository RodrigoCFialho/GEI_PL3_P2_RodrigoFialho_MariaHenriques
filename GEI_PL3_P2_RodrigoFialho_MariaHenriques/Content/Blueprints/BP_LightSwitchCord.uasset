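; BP_LightSwitchCord is a light switch cord that becomes usable once blockades are cleared and then triggers a level change.
; Its BlockadeDestroyed event counts calls and, on the second, shows both cylinders and enables collision on one.
; The Turn override calls its parent, then Interact, which invokes BPI_Activable's ToggleActivation on itself.
; ToggleActivation calls ChangeLevel on the GI_BatteryKeeper game instance only if the cord has been revealed.
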(event `Blockade Destroyed`
  (bind _output_get (set `self.NumberOfBlockades` (+ (`self.NumberOfBlockades`) 1)))
  (if (== _output_get 2)
    (`SceneComponent.SetVisibility` (`self.Cylinder`) true false)
    (`SceneComponent.SetVisibility` (`self.Cylinder1`) true false)
    (`PrimitiveComponent.SetCollisionEnabled` (`self.Cylinder1`) "QueryAndPhysics")
    (set `self.bIsVisible` true)))

(event `/Game/Blueprints/BPI_Activable.ToggleActivation`
  (params (bActivate :type Boolean))
  (if (`self.bIsVisible`)
    (bind _asgi_battery_keeper (cast `/Game/Blueprints/GameInstance/GI_BatteryKeeper` (`GameplayStatics.GetGameInstance`)))
    (`/Game/Blueprints/GameInstance/GI_BatteryKeeper.Change Level` _asgi_battery_keeper)))

(fn `Turn`
  (params (bOn :type Boolean))
  (`parent.Turn` bOn)
  (`self.Interact` bOn))

(fn `UserConstructionScript`)