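; Game instance that holds the battery count and handles level changes through a ChangeLevel event.
; From Level1 it opens Level2; from any other level it resets the count to zero and opens MainMenu.
; Both branches copy the count to the player's BP_MainCharacter immediately after the open-level call, so the write targets the current pawn, before the new level loads.
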(event `Change Level`
  (bind _returnvalue (`GameplayStatics.GetCurrentLevelName` true))
  (if (`KismetStringLibrary.EqualEqual_StrStr` _returnvalue "Level1")
    (`GameplayStatics.OpenLevel` "Level2")
    (bind _asbp_main_character (cast `/Game/Characters/Characters/Main/BP_MainCharacter` (`GameplayStatics.GetPlayerPawn` 0)))
    (set `/Game/Characters/Characters/Main/BP_MainCharacter.BatteryNumber` (`self.BatteryNumber`) _asbp_main_character)
    (else
      (`GameplayStatics.OpenLevel` "MainMenu")
      (bind _output_get (set `self.BatteryNumber` 0))
      (bind _asbp_main_character_2 (cast `/Game/Characters/Characters/Main/BP_MainCharacter` (`GameplayStatics.GetPlayerPawn` 0)))
      (set `/Game/Characters/Characters/Main/BP_MainCharacter.BatteryNumber` _output_get _asbp_main_character_2))))