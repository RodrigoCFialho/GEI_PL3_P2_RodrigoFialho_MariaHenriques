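; BP_VoidOrb is a one-use, battery-powered orb that can activate a linked Blockade and then dissolves.
; ToggleActivation checks the main character's battery count, printing a message at zero, otherwise calling Turn and fading the Sphere's Opacity through a timeline before destroying the actor.
; On its first call only, Turn runs the parent logic and Interact, which removes a battery and toggles the Blockade via BPI_Activable.
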(event `/Game/Blueprints/BPI_Activable.ToggleActivation`
  (params (bActivate :type Boolean))
  (bind _asbp_main_character (cast `/Game/Characters/Characters/Main/BP_MainCharacter` (`GameplayStatics.GetPlayerPawn` 0)))
  (if (!= (`/Game/Characters/Characters/Main/BP_MainCharacter.BatteryNumber` _asbp_main_character) 0)
    (`self.Turn` true)
    (bind (_direction _dissolve) (`Timeline|Dissolve` :!via `PlayFromStart`)
      (:`Update`
        (`MeshComponent.SetScalarParameterValueOnMaterials` (`self.Sphere`) "Opacity" _dissolve))
      (:`Finished`
        (`self.K2_DestroyActor`)))
    (else
      (`KismetSystemLibrary.PrintText` "You have 0 batteries"))))

(fn `Turn`
  (params (bOn :type Boolean))
  (bind _output_get (set `self.NumberOfInteractions` (+ (`self.NumberOfInteractions`) 1)))
  (if (== _output_get 1)
    (`parent.Turn` bOn)
    (`self.Interact` bOn)))

(fn `UserConstructionScript`)